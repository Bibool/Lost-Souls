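; Toxic bubble actor that bobs its static mesh vertically in an endless loop from BeginPlay.
; A timed MoveComponentTo shifts the mesh up or down by a fixed offset from its current relative location, chosen by the REset flag.
; After each move, a FlipFlop alternately clears or sets that flag and loops back into the next move, so no Tick is needed.
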(event EventBeginPlay
  (bind _staticmeshcomponent0 (Variables|Default|GetStaticMeshComponent0))
  (bind _relativelocation (Variables|/Script/Engine.SceneComponent|GetRelativeLocation _staticmeshcomponent0))
  (Components|MoveComponentTo _staticmeshcomponent0 (Math|Vector|SelectVector (+ _relativelocation "0, 0,75.000000") (+ _relativelocation "0.000000, 0,-75.000000") (Variables|Default|GetREset)) "0, 0, 0" false false 4.0 false :!label _label)
  (Utilities|FlowControl|FlipFlop
    (:A
      (Variables|Default|SetREset false)
      (goto _label))
    (:B
      (Variables|Default|SetREset true)
      (goto _label))))

(event Collision|EventActorBeginOverlap
  (params (OtherActor :type Actor%20Object%20Reference)))

(event EventTick
  (params (DeltaSeconds :type Float%20%28single-precision%29)))

(fn ConstructionScript
  (|CallParentFunction))