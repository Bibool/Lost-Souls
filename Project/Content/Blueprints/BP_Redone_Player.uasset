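; Player character Blueprint that adds the crosshair HUD, controls music and handles death.
; Overlapping a Musictrigger messages overlapped Interact_I actors, crossfades to combat music and plays the mural level sequence once.
; When the sequence first stops, the camera blends back to the pawn.
; On death, it stops music, plays a death sound, ragdolls the mesh and fades in a retry screen via timeline before pausing.
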(event Custom|FadeInDeathScreen
  (params (DeathInterface :type Bp%20Death%20Interface%20Object%20Reference))
  (bind _returnvalue (Game|GetPlayerController 0))
  (UserInterface|Viewport|AddtoViewport DeathInterface 0)
  (Input|SetInputModeUIOnly _returnvalue (Variables|/Game/Blueprints/UI/Bp_DeathInterface.Bp_DeathInterface_C|GetRetryBtn DeathInterface) "DoNotLock")
  (bind _opacity (Timeline|Timeline_0 PlayFromStart)
    (:Update
      (Appearance|SetColorandOpacity DeathInterface (Utilities|Struct|MakeLinearColor 1.0 1.0 1.0 _opacity) :!class /Script/UMG.UserWidget)
      (Physics|SetSimulatePhysics (Variables|Character|GetMesh) true)
      (Variables|/Script/Engine.PlayerController|SetbShowMouseCursor _returnvalue true))
    (:Finished
      (Game|SetGamePaused true))))

(event Custom|CustomEvent_0
  (Utilities|FlowControl|DoOnce false
    (:Completed
      (Game|Player|SetViewTargetwithBlend (Game|GetPlayerController 0) (Game|Player|GetPlayerPawn 0) 0.5 "VTBlend_EaseOut" 0.0 true))))

(event EventBeginPlay
  (bind _returnvalue (UserInterface|CreateWidget "/Game/Blueprints/UI/WBP_CrossHair.WBP_CrossHair_C"))
  (UserInterface|Viewport|AddtoViewport _returnvalue 0)
  (Audio|Components|Audio|SetSound (Variables|Default|GetAudio) "/Game/Audio/GameAudio/Water_Temple_.Water_Temple_"))

(event EventOnDeathBP
  ;[1 1 1] Death from enemy damage
  (CallFunction|KillPlayer))

(event Collision|EventActorBeginOverlap
  (params (OtherActor :type Actor%20Object%20Reference))
  (bind _audio (Variables|Default|GetAudio))
  (Utilities|Casting|CastToMusictrigger OtherActor)
  (Utilities|FlowControl|Sequence
    (:then_0
      (bind _outactors (Actor|GetAllActorswithInterface "/Game/Maps/Level_Designer/Dialogue/Interact_I.Interact_I_C"))
      (for _array_element _outactors
        (if (Collision|IsOverlappingActor _array_element self :!class /Script/Engine.Actor)
          (Class|InteractI|Interact(Message) _array_element))))
    (:then_1
      (Audio|Components|Audio|FadeOut (Variables|Default|GetAudio) 2.0 0.0 "Linear" :!class /Script/Engine.AudioComponent)
      (Audio|Components|Audio|SetSound _audio "/Game/Combat_uni.Combat_uni")
      (Audio|Components|Audio|FadeIn _audio 2.0 1.0 0.0 "Linear" :!class /Script/Engine.AudioComponent)
      (if (not (Variables|Default|GetMuralSequence))
        (bind _outactor (Sequencer|Player|CreateLevelSequencePlayer "/Game/LevelSequence/MuralSequence.MuralSequence"))
        (Sequencer|Player|Play (Variables|/Script/LevelSequence.LevelSequenceActor|GetSequencePlayer _outactor) :!class /Script/MovieScene.MovieSceneSequencePlayer)
        (Variables|Default|SetMuralSequence true)
        (EventDispatchers|BindEventtoOnStop (Variables|/Script/LevelSequence.LevelSequenceActor|GetSequencePlayer _outactor) (delegate Custom|CustomEvent_0))))))

(fn ConstructionScript)

(fn KillPlayer
  (bind _returnvalue (UserInterface|CreateWidget "/Game/Blueprints/UI/Bp_DeathInterface.Bp_DeathInterface_C" (Game|GetPlayerController 0)))
  (bind _output_get (Variables|Default|SetDeathinterface _returnvalue))
  (CallFunction|FadeinDeathScreen _output_get)
  (Audio|Components|Audio|Stop (Variables|Default|GetAudio))
  (Audio|PlaySoundatLocation "/Game/Sounds/deathaudio.deathaudio" (Transformation|GetWorldLocation (Variables|Default|GetCapsuleComponent)) "0, 0, 0" 1.0 1.0 0.0 0 0 0))

(fn StopAudio
  (Audio|Components|Audio|SetSound (Variables|Default|GetAudio) "/Game/Blueprints/UI/UIImages/beep.beep"))